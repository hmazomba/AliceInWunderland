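; AI controller for an NPC that keeps moving toward locations supplied by GetPlayerLocation, starting on BeginPlay.
; GotoLocation runs AI MoveTo to a random reachable point near the target.
; Success requests a new location and sends it through a GoToLocation message, while failure retries after a short delay, forming an endless movement loop.
; The getPlayerLocation graph holds only an unused random-point node around the controlled pawn, with no player lookup shown.
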(event `self.ReceiveBeginPlay`
  (`self.GoToLocation` (`self.getPlayerLocation` 600.0)))

(event `self.GoToLocation`
  (params (TargetLocation :type "Vector Structure"))
  (`|AIMoveTo` null (`NavigationSystemV1.K2_GetRandomReachablePointInRadius` TargetLocation 300.0 null null) null 200.0 :!label _label
    (:`OnSuccess`
      (message `/Game/Wunderland/Core/Blueprints/AI/BPI_AI.GoToLocation` self (`self.getPlayerLocation` 200.0)))
    (:`OnFail`
      (`KismetSystemLibrary.Delay` 3.0)
      (goto _label))))

(fn `UserConstructionScript`)